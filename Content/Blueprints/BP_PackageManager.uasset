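; BP_PackageManager manages the BP_PackagePoints actors in the level, keeping one randomly chosen point visible and active at a time.
; On BeginPlay it caches every point of that class through GetPoints.
; SelectNewPoint re-rolls until it draws an inactive point, then hides and deactivates all points before showing and activating the new one.
; Nothing in this Blueprint calls SelectNewPoint.
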(event `self.ReceiveBeginPlay`
  (`self.GetPoints`))

(event `GetPoints`
  (bind _outactors (`GameplayStatics.GetAllActorsOfClass` "/Game/Blueprints/BP_PackagePoints.BP_PackagePoints_C"))
  (set `self.Points` _outactors))

(event `SelectNewPoint`
  (bind _points (`self.Points`))
  (bind _selected (`self.Selected`))
  (bind _output_get (set `self.Selected` (`KismetArrayLibrary.Array_Random` _points) :!label _label))
  (if (`/Game/Blueprints/BP_PackagePoints.Active` _output_get)
    (goto _label)
    (else
      (for _array_element _points
        (`self.SetActorHiddenInGame` _array_element true)
        (set `/Game/Blueprints/BP_PackagePoints.Active` false _array_element))
      (`self.SetActorHiddenInGame` _selected false)
      (set `/Game/Blueprints/BP_PackagePoints.Active` true _selected))))

(fn `UserConstructionScript`)