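; Road intersection actor that tracks connected BP_Roads, manages their traffic lights and supplies random next roads.
; The construction script and UpdateRoads rebuild RoadsInfo from DetectorBox overlaps, using "end" component tags for drive direction.
; SpawnTrafficLights places direction-oriented lights with staggered start delays; DestroyLights removes every traffic light in the level.
; GetRandomNextRoad loops until a roll differs from the origin, but re-rolls on return, so can still return it.
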(event `UpdateRoads`
  (bind _detectorbox (`self.DetectorBox`))
  (`KismetArrayLibrary.Array_Clear` (`self.RoadsInfo`))
  (bind _outcomponents (`KismetSystemLibrary.ComponentOverlapComponents` _detectorbox (`SceneComponent.K2_GetComponentToWorld` _detectorbox) (`|MakeArray` "ObjectTypeQuery1" :!type "EObjectTypeQuery Enum") "/Script/Engine.BoxComponent"))
  (for _array_element _outcomponents
    (bind _asbp_roads (cast `/Game/Blueprints/BP_Roads` (`ActorComponent.GetOwner` _array_element)))
    (bind _returnvalue (`self.SetRoadInfo` _asbp_roads (not (`ActorComponent.ComponentHasTag` _array_element "end"))))
    (`KismetArrayLibrary.Array_Add` (`self.RoadsInfo`) _returnvalue)))

(event `SpawnTrafficLights`
  (for (_array_element _array_index) (`self.RoadsInfo`)
    (bind (_road _boneweyroad _broaddrivesforward) (break `DDRoadInfo` _array_element))
    (bind _returnvalue (`self.K2_GetActorRotation` _road))
    (bind _returnvalue_2 (`|SpawnActorFromClass` "/Game/Blueprints/BP_TrafficLight.BP_TrafficLight_C" (`KismetMathLibrary.MakeTransform` (+ (+ (`self.K2_GetActorLocation`) (0.0 0.0 300.0)) (* (`KismetMathLibrary.GetForwardVector` _returnvalue) (`KismetMathLibrary.SelectFloat` 800.0 (* 800.0 -1.0) _broaddrivesforward))) (`KismetMathLibrary.SelectRotator` _returnvalue (`KismetMathLibrary.MakeRotator` (.roll _returnvalue) (.pitch _returnvalue) (+ (.yaw _returnvalue) 180.0)) _broaddrivesforward)) "Undefined" "OverrideRootScale" null null))
    (set `/Game/Blueprints/BP_TrafficLight.InitialDelay` (* _array_index 10.0) _returnvalue_2)))

(event `Destroy Lights`
  (bind _outactors (`GameplayStatics.GetAllActorsOfClass` "/Game/Blueprints/BP_TrafficLight.BP_TrafficLight_C"))
  (for _array_element _outactors
    (`self.K2_DestroyActor` _array_element)))

(fn `GetRandomNextRoad`
  (params (OriginRoad :type "DDRoad Object Reference"))
  (returns (Output :type "DDRoadInfo Structure"))
  (bind _returnvalue (`KismetArrayLibrary.Array_Length` (`self.RoadsInfo`)))
  (bind _output (`|GetArrayItem` (`self.RoadsInfo`) (`KismetMathLibrary.RandomInteger` _returnvalue)))
  (if (> _returnvalue 1)
    (while (== (`.Road` (break `DDRoadInfo` _output)) OriginRoad)
      (`KismetSystemLibrary.PrintString` "Is equal"))
    (return _output)))

(fn `UserConstructionScript`
  (bind _detectorbox (`self.DetectorBox`))
  (`KismetArrayLibrary.Array_Clear` (`self.RoadsInfo`))
  (bind _outcomponents (`KismetSystemLibrary.ComponentOverlapComponents` _detectorbox (`SceneComponent.K2_GetComponentToWorld` _detectorbox) (`|MakeArray` "ObjectTypeQuery1" :!type "EObjectTypeQuery Enum") "/Script/Engine.BoxComponent"))
  (for _array_element _outcomponents
    (bind _asbp_roads (cast `/Game/Blueprints/BP_Roads` (`ActorComponent.GetOwner` _array_element)))
    (bind _returnvalue (`self.SetRoadInfo` _asbp_roads (not (`ActorComponent.ComponentHasTag` _array_element "end"))))
    (`KismetArrayLibrary.Array_Add` (`self.RoadsInfo`) _returnvalue)))