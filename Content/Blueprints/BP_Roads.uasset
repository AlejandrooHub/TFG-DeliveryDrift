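; BP_Roads is a spline-based road actor whose construction script keeps its endpoint markers aligned to the spline.
; A box and an arrow sit slightly raised at both the start and end, following the spline's rotation, with the arrows yawed a quarter turn from it.
; A separate Arrow component's length scales with the end marker's distance from the actor's local origin.
; The event graph holds no runtime logic.
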(fn `UserConstructionScript`
  (bind _splinecomponent (`self.SplineComponent`))
  (bind _returnvalue (`SplineComponent.GetSplineLength` _splinecomponent))
  (bind _returnvalue_2 (`SplineComponent.GetRotationAtDistanceAlongSpline` _splinecomponent 0.0 "Local"))
  (bind _returnvalue_3 (`SplineComponent.GetRotationAtDistanceAlongSpline` _splinecomponent _returnvalue "Local"))
  (bind _returnvalue_4 (+ (`SplineComponent.GetLocationAtDistanceAlongSpline` _splinecomponent 0.0 "Local") (0.0 0.0 100.0)))
  (bind _returnvalue_5 (+ (`SplineComponent.GetLocationAtDistanceAlongSpline` _splinecomponent _returnvalue "Local") (0.0 0.0 100.0)))
  (`SceneComponent.K2_SetRelativeLocationAndRotation` (`self.BoxEnd`) _returnvalue_5 _returnvalue_3 false false)
  (`SceneComponent.K2_SetRelativeLocationAndRotation` (`self.ArrowEnd`) _returnvalue_5 (`KismetMathLibrary.MakeRotator` (.roll _returnvalue_3) (.pitch _returnvalue_3) (+ (.yaw _returnvalue_3) 90.0)) false false)
  (`SceneComponent.K2_SetRelativeLocationAndRotation` (`self.BoxStart`) _returnvalue_4 _returnvalue_2 false false)
  (`SceneComponent.K2_SetRelativeLocationAndRotation` (`self.ArrowStart`) _returnvalue_4 (`KismetMathLibrary.MakeRotator` (.roll _returnvalue_2) (.pitch _returnvalue_2) (+ (.yaw _returnvalue_2) 90.0)) false false)
  (set `ArrowComponent.ArrowLength` (/ (`KismetMathLibrary.VSize` (`SceneComponent.RelativeLocation` (`self.ArrowEnd`))) 20.0) (`self.Arrow`)))