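; AI-driven car that follows road splines in traffic, picks random roads at intersections and kills cyclists it touches.
; A looping timer re-syncs its spline target from the nearest point, and Tick advances that target when close.
; Steering corrects the error between a five-step velocity-extrapolated position and the target.
; Throttle follows a max speed set by heading error, slowing near road ends and braking for non-green lights.
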(event `BindToRoad`
  (bind _outactors (`GameplayStatics.GetAllActorsOfClass` "/Game/Blueprints/BP_Roads.BP_Roads_C"))
  (bind _asddroad (cast `DDRoad` (`.ReturnValue` (`GameplayStatics.FindNearestActor` (`self.K2_GetActorLocation`) _outactors))))
  (bind _output_get (set `self.Road` _asddroad))
  (set `self.RoadSpline` (`DDRoad.SplineComponent` _output_get)))

(event `self.ReceiveBeginPlay`
  (`parent.ReceiveBeginPlay`)
  (if (`self.Activated`)
    (`KismetSystemLibrary.K2_SetTimerDelegate` (delegate `FindNextTarget_Event`) 0.3 true)
    (bind _road (`self.Road`)
      (:`then`
        (set `self.RoadSpline` (`DDRoad.SplineComponent` _road)))
      (:`else`))
    (else
      (`KismetSystemLibrary.PrintString` (`KismetStringLibrary.Concat_StrStr` (`KismetSystemLibrary.GetDisplayName` self) ": No activadoooooooo")))))

(event `FindNextTarget_Event`
  (`self.FindNextTarget`))

(event `self.ReceiveTick`
  (params (DeltaSeconds :type "Float (single-precision)"))
  (bind _roadspline (`self.RoadSpline`))
  (bind _targetsplinedistance (`self.TargetSplineDistance`))
  (bind _roadspline_2 (`self.RoadSpline`))
  (bind _returnvalue (`KismetMathLibrary.SelectFloat` 1.0 -1.0 (`self.DriveOnRight`)))
  (bind (_returnvalue_roll _returnvalue_pitch _returnvalue_yaw) (`KismetMathLibrary.BreakRotator` (`KismetMathLibrary.NormalizedDeltaRotator` (`KismetMathLibrary.FindLookAtRotation` (`self.K2_GetActorLocation`) (`self.TargetPoint`)) (`self.K2_GetActorRotation`))))
  (bind _returnvalue_2 (/ 500.0 (`KismetMathLibrary.Abs` _returnvalue_yaw)))
  (bind _returnvalue_3 (< (`KismetMathLibrary.Vector_Distance` (`self.K2_GetActorLocation`) (`SplineComponent.GetLocationAtDistanceAlongSpline` _roadspline_2 (`KismetMathLibrary.SelectFloat` (`SplineComponent.GetSplineLength` _roadspline_2) 0.0 (`self.DrivingForward`)) "World")) 1000.0))
  (`parent.ReceiveTick` DeltaSeconds)
  (if (`self.Activated`)
    (`self.SpeedControl`)
    (bind _output_get (set `self.MaxSpeed` (`KismetMathLibrary.SelectFloat` 0.0 (`KismetMathLibrary.FClamp` (`KismetMathLibrary.Lerp` (`self.MaxSpeed`) _returnvalue_2 (* (`GameplayStatics.GetWorldDeltaSeconds`) (`KismetMathLibrary.SelectFloat` 20.0 1.0 (> (`self.MaxSpeed`) _returnvalue_2)))) 10.0 30.0) _returnvalue_3)))
    (if (not _returnvalue_3)
      _
      (elif (not (not (> (* (`KismetMathLibrary.Abs` (`ChaosVehicleMovementComponent.GetForwardSpeed` (`self.VehicleMovementComponent`))) 0.036) 12.0)))
        (`self.Brake` 0.01)))
    (bind _output_get_2 (set `self.TargetPoint` (+ (`SplineComponent.GetLocationAtDistanceAlongSpline` _roadspline _targetsplinedistance "World") (* (`SplineComponent.GetRightVectorAtDistanceAlongSpline` _roadspline _targetsplinedistance "World") (* (`self.LaneWidth`) (`KismetMathLibrary.SelectFloat` _returnvalue (* _returnvalue -1.0) (`self.DrivingForward`)))))))
    (if (< (`KismetMathLibrary.Vector_Distance` (`self.TargetPoint`) (`self.K2_GetActorLocation`)) (`self.CheckGap`))
      (`self.SetSplineDistance`))
    (`self.PredictPath`)))

(event `self.PreCollisionDetector.OnComponentEndOverlap`
  (params (OverlappedComponent :type "PrimitiveComponent Object Reference") (OtherActor :type "Actor Object Reference") (OtherComp :type "PrimitiveComponent Object Reference") (OtherBodyIndex :type Integer))
  (`|ExecutionSequence`
    (:`then_1`
      (cast `/Game/Blueprints/AI_Car` OtherActor)
      (set `self.InconmingCollision` false))))

(event `self.PreCollisionDetector.OnComponentBeginOverlap`
  (params (OverlappedComponent :type "PrimitiveComponent Object Reference") (OtherActor :type "Actor Object Reference") (OtherComp :type "PrimitiveComponent Object Reference") (OtherBodyIndex :type Integer) (bFromSweep :type Boolean) (SweepResult :type "HitResult Structure (by ref)"))
  (`|ExecutionSequence`
    (:`then_0`
      (bind _asbp_intersection (cast `/Game/Blueprints/BP_Intersection` OtherActor))
      (`KismetSystemLibrary.PrintString` "Entered Intersection" true true (struct :`R` 0.226841 :`G` 1.0 :`A` 1.0))
      (bind _output (`/Game/Blueprints/BP_Intersection.GetRandomNextRoad` _asbp_intersection (`self.Road`)))
      (bind (_road _boneweyroad _broaddrivesforward) (break `DDRoadInfo` _output))
      (bind _output_get (set `self.Road` _road))
      (set `self.RoadSpline` (`DDRoad.SplineComponent` _output_get))
      (bind _output_get_2 (set `self.DrivingForward` _broaddrivesforward))
      (set `self.TargetSplineDistance` (`KismetMathLibrary.SelectFloat` 0.0 (`SplineComponent.GetSplineLength` (`self.RoadSpline`)) _output_get_2)))))

(event `self.Car Boundaries.OnComponentBeginOverlap`
  (params (OverlappedComponent :type "PrimitiveComponent Object Reference") (OtherActor :type "Actor Object Reference") (OtherComp :type "PrimitiveComponent Object Reference") (OtherBodyIndex :type Integer) (bFromSweep :type Boolean) (SweepResult :type "HitResult Structure (by ref)"))
  (bind _asbp_cyclist (cast `/Game/Character/BP_Cyclist` OtherActor))
  (`/Game/Character/BP_Cyclist.Die` _asbp_cyclist))

(event `self.PreLightDetector.OnComponentBeginOverlap`
  (params (OverlappedComponent :type "PrimitiveComponent Object Reference") (OtherActor :type "Actor Object Reference") (OtherComp :type "PrimitiveComponent Object Reference") (OtherBodyIndex :type Integer) (bFromSweep :type Boolean) (SweepResult :type "HitResult Structure (by ref)"))
  (bind _asbp_traffic_light (cast `/Game/Blueprints/BP_TrafficLight` OtherActor))
  (set `self.TrafficLight` _asbp_traffic_light))

(event `self.PreLightDetector.OnComponentEndOverlap`
  (params (OverlappedComponent :type "PrimitiveComponent Object Reference") (OtherActor :type "Actor Object Reference") (OtherComp :type "PrimitiveComponent Object Reference") (OtherBodyIndex :type Integer))
  (`|ExecutionSequence`
    (:`then_0`
      (cast `/Game/Blueprints/BP_TrafficLight` OtherActor)
      (set `self.TrafficLight` (`self.ResetTrafficLight`)))))

(fn `FindNextTarget`
  (locals (SplineDistance :type "Float (double-precision)") (DistanceToClosestPoint :type "Float (double-precision)" :default 1000000000.0) (ClosestPointSplineDistance :type "Float (double-precision)"))
  (bind _splinedistance (`local.SplineDistance`))
  (bind _closestpointsplinedistance (`local.ClosestPointSplineDistance`))
  (bind _returnvalue (`SplineComponent.GetSplineLength` (`self.RoadSpline`)))
  (bind _returnvalue_2 (- _closestpointsplinedistance 1000.0))
  (bind _returnvalue_3 (+ _closestpointsplinedistance 1000.0))
  (bind _returnvalue_4 (`KismetMathLibrary.Vector_Distance` (`SplineComponent.GetLocationAtDistanceAlongSpline` (`self.RoadSpline`) (`local.SplineDistance`) "World") (`self.K2_GetActorLocation`)))
  (if (< _returnvalue_4 (`local.DistanceToClosestPoint`)) :!label _label
    (set `local.DistanceToClosestPoint` _returnvalue_4)
    (set `local.ClosestPointSplineDistance` _splinedistance))
  (bind _output_get (set `local.SplineDistance` (+ _splinedistance 200.0)))
  (if (> _output_get _returnvalue)
    (if (`self.DrivingForward`)
      (set `self.TargetSplineDistance` (`KismetMathLibrary.SelectFloat` 0.0 _returnvalue_3 (> _returnvalue_3 _returnvalue)))
      (else
        (set `self.TargetSplineDistance` (`KismetMathLibrary.SelectFloat` _returnvalue _returnvalue_2 (< _returnvalue_2 0.0)))))
    (else
      (goto _label))))

(fn `PredictPath`
  (locals (PredictedLocation :type "Vector Structure") (Velocity :type "Vector Structure") (TimeStep :type "Float (double-precision)") (SteerYaw :type "Float (double-precision)"))
  (bind _returnvalue (`self.K2_GetActorLocation`))
  (bind _returnvalue_2 (`self.K2_GetActorLocation`))
  (bind (_returnvalue_roll _returnvalue_pitch _returnvalue_yaw) (`KismetMathLibrary.BreakRotator` (`KismetMathLibrary.NormalizedDeltaRotator` (`KismetMathLibrary.FindLookAtRotation` _returnvalue_2 (`local.PredictedLocation`)) (`KismetMathLibrary.FindLookAtRotation` _returnvalue_2 (`self.TargetPoint`)))))
  (bind (_returnvalue_roll_2 _returnvalue_pitch_2 _returnvalue_yaw_2) (`KismetMathLibrary.BreakRotator` (`KismetMathLibrary.NormalizedDeltaRotator` (`KismetMathLibrary.Conv_VectorToRotator` (`KismetMathLibrary.Normal` (`local.Velocity`))) (`self.K2_GetActorRotation`))))
  (set `local.PredictedLocation` _returnvalue)
  (set `local.Velocity` (`self.GetVelocity`))
  (set `local.TimeStep` (/ (/ (`KismetMathLibrary.Vector_Distance` _returnvalue (`self.TargetPoint`)) (`KismetMathLibrary.VSize` (`local.Velocity`))) 5.0))
  (set `local.SteerYaw` _returnvalue_yaw_2)
  (for _ (range 1 6)
    (set `local.PredictedLocation` (+ (`local.PredictedLocation`) (* (`local.Velocity`) (`local.TimeStep`))))
    (set `local.Velocity` (`KismetMathLibrary.RotateAngleAxis` (`local.Velocity`) (`local.SteerYaw`) (0.0 0.0 1.0))))
  (bind _output_get (set `self.SteerAmount` (`KismetMathLibrary.FClamp` (* _returnvalue_yaw -0.1) -1.0)))
  (`self.Steer` _output_get))

(fn `UserConstructionScript`
  (`parent.UserConstructionScript`)
  (bind _road (`self.Road`)
    (:`then`
      (set `self.RoadSpline` (`DDRoad.SplineComponent` _road)))
    (:`else`)))